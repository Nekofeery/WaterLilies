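; BP_WaterLily is a water lily flower actor that responds to mouse hover and clicks.
; On BeginPlay it caches the MyPawn instance as ActivePawn.
; Cursor and click events query the pawn's active mode and pass it to BeginHover or WasClicked, the latter also receiving the pawn's SpawnedActors, while cursor exit calls EndHover.
; The construction script assigns the FlowerPetals component as PetalMeshComponent.
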(event EventBeginPlay
  (bind _returnvalue (Actor|GetActorOfClass "/Script/WaterLilies.MyPawn"))
  (Variables|Default|SetActivePawn _returnvalue))

(event MouseInput|EventActorBeginCursorOver
  (bind _returnvalue (Class|MyPawn|GetActiveMode (Variables|Default|GetActivePawn)))
  (Class|WaterLilyActor|BeginHover _returnvalue))

(event MouseInput|EventActorEndCursorOver
  (Class|MyPawn|GetActiveMode (Variables|Default|GetActivePawn))
  (Class|WaterLilyActor|EndHover))

(event MouseInput|EventActorOnClicked
  (params (ButtonPressed :type Key%20Structure :default "None"))
  (bind _activepawn (Variables|Default|GetActivePawn))
  (bind _returnvalue (Class|MyPawn|GetActiveMode _activepawn))
  (Class|WaterLilyActor|WasClicked _returnvalue (Variables|/Script/WaterLilies.MyPawn|GetSpawnedActors _activepawn)))

(fn ConstructionScript
  (Variables|Default|SetPetalMeshComponent (Variables|Default|GetFlowerPetals)))